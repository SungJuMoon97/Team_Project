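; Asteroid ring actor that fills a circular band with instanced meshes and spins around its Z axis on Tick.
; The construction script sets mesh and cull distances on a hierarchical instanced static mesh component, then adds instances in a length-by-width loop.
; AsteroidTransformation places each around the ring using TransformRandom stream jitter, blending ring-aligned rotation toward random.
; Scale grows with width index rather than being random, leaving the first row at zero.
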(event EventTick
  (params (DeltaSeconds :type Float%20%28single-precision%29))
  (Transformation|AddActorLocalRotation (Math|Vector|RotatorfromAxisandAngle "0, 0,1.000000" (* DeltaSeconds (Variables|Animation|GetRotationSpeed))) false false))

(fn ConstructionScript
  (bind _hierarchicalinstancedstaticspawn (Variables|Default|GetHierarchicalInstancedStaticSpawn))
  (bind _instancecountbylength (Variables|인스턴스|GetInstanceCountByLength))
  (bind _instancecountbywidth (Variables|Instances|GetInstanceCountByWidth))
  (Utilities|FlowControl|Sequence
    (:then_0
      (Components|StaticMesh|SetStaticMesh _hierarchicalinstancedstaticspawn (Variables|Instances|GetInstanceMesh)))
    (:then_1
      (Components|InstancedStaticMesh|SetCullDistances _hierarchicalinstancedstaticspawn (Variables|Perfcrmance|GetCullingNear) (Variables|Perfcrmance|GetCullingFar)))
    (:then_2
      (for _index (range 0 (- _instancecountbylength 1))
        (for _index_2 (range 0 (- _instancecountbywidth 1))
          (bind (_out_location _out_rotating) (CallFunction|AsteroidTransformation _index_2 _instancecountbywidth _index _instancecountbylength))
          (Components|InstancedStaticMesh|AddInstance (Variables|Default|GetHierarchicalInstancedStaticSpawn) (Math|Transform|MakeTransform _out_location _out_rotating (Math|Conversions|ToVector(Float) (* _index_2 (Variables|Transform|GetRandomScaleMinimum)))) false))))))

(fn AsteroidTransformation
  (params (Index%20From%20Width%20Loop :type Integer) (Number%20Of%20Instances%20By%20Width :type Integer) (Index%20from%20Length%20Loop :type Integer) (Number%20Of%20Instances%20By%20Length :type Integer))
  (bind _returnvalue (Math|Vector|MakeVector 0.0 0.0 1.0))
  (bind _returnvalue_2 (Math|Conversions|ToFloat(Integer) Number%20Of%20Instances%20By%20Length))
  (bind _returnvalue_3 (Math|Conversions|ToFloat(Integer) Index%20from%20Length%20Loop))
  (bind _returnvalue_4 (Math|Conversions|ToFloat(Integer) Number%20Of%20Instances%20By%20Width))
  (bind _returnvalue_5 (Math|Conversions|ToFloat(Integer) Index%20From%20Width%20Loop))
  (bind _returnvalue_6 (Math|Float|MakeLiteralFloat 3.6e+02))
  (bind _transformrandom (Variables|Transform|GetTransformRandom))
  (bind _randomizeposition (Variables|Transform|GetRandomizePosition))
  (bind _randomizezaxisposit (Variables|Transform|GetRandomizeZAxisPosit))
  (bind _ringwidth (Variables|인스턴스|GetRingWidth))
  (bind _ringwidth_2 (Variables|인스턴스|GetRingWidth))
  (bind _ringradius (Variables|인스턴스|GetRingRadius))
  (bind _returnvalue_7 (Math|Random|RandomFloatfromStream _transformrandom))
  (bind _returnvalue_8 (Math|Random|RandomUnitVectorfromStream _transformrandom))
  (bind _returnvalue_9 (/ _returnvalue_3 _returnvalue_2))
  (bind _returnvalue_10 (/ _returnvalue_5 _returnvalue_4))
  (bind _returnvalue_11 (- _returnvalue_7 0.5))
  (bind _returnvalue_12 (* _returnvalue_8 _randomizeposition))
  (bind _returnvalue_13 (- _returnvalue_10 0.5))
  (bind _returnvalue_14 (* _returnvalue_9 _returnvalue_6))
  (bind _returnvalue_15 (* _returnvalue_11 _randomizezaxisposit _ringwidth))
  (bind _returnvalue_16 (* _returnvalue_13 _ringwidth_2))
  (bind _returnvalue_17 (+ _ringradius _returnvalue_16))
  (bind _returnvalue_18 (+ _returnvalue_15 _returnvalue_12))
  (bind _returnvalue_19 (Math|Vector|MakeVector 0.0 _returnvalue_17 0.0))
  (bind _returnvalue_20 (+ _returnvalue_18 _returnvalue_19))
  (bind _returnvalue_21 (Math|Vector|RotateVectorAroundAxis _returnvalue_20 _returnvalue_14 _returnvalue))
  (return _returnvalue_21 (Math|Rotator|Lerp(Rotator) (Class|KismetMathLibrary|MakeRotfromYZ (Math|Vector|CrossProduct _returnvalue _returnvalue_21) _returnvalue) (Class|KismetMathLibrary|RandomRotatorfromStream true (Variables|Transform|GetTransformRandom)) (Variables|Transform|GetRandomizeRotation) true)))