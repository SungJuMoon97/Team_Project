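; Menu3D_BP is a 3D menu actor that hosts a Menu3D_Widget and transitions the player's view between linked menu actors.
; On BeginPlay it binds to the widget's transition event, which passes an index into its LinkedMenu array.
; A valid index disables collision on this menu, enables it on the target, and eases player 0's view target to that menu with a timed blend.
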(event Custom|TransitionTo
  (params (NewMenu :type Menu%203D%20BP%20Object%20Reference))
  (Collision|SetActorEnableCollision false)
  (Collision|SetActorEnableCollision NewMenu true)
  (Game|Player|SetViewTargetwithBlend (Game|GetPlayerController 0) NewMenu 2.0 "VTBlend_EaseInOut" 2.0 false))

(event Custom|OnTransitionBetweenMenus
  (params (MenuIndex :type Integer))
  (if (Utilities|Array|IsValidIndex (Variables|Default|GetLinkedMenu) MenuIndex)
    (CallFunction|Transitionto (Utilities|Array|Get(acopy) (Variables|Default|GetLinkedMenu) MenuIndex))))

(event EventBeginPlay
  (bind _asmenu_3d_widget (Utilities|Casting|CastToMenu3D_Widget (UserInterface|GetUserWidgetObject (Variables|Default|GetWidget))))
  (EventDispatchers|BindEventtoTransitiontoLinkedMenu _asmenu_3d_widget (delegate Custom|OnTransitionBetweenMenus)))

(fn ConstructionScript)